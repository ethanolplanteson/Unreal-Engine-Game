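; NPC pawn Blueprint for random wandering on the navmesh.
; The Move event picks a reachable point around the actor and runs AI MoveTo, then calls MoveNPC after a pause on success or a brief retry delay on failure.
; BeginPlay also calls MoveNPC, but that function is empty and nothing here triggers Move.
; GetInvertMultiplier returns a sign from ToggleInvert and is unused here.
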(event Custom|Move
  (bind _output_get (Variables|Default|SetRandom%20Location (.RandomLocation (AI|Navigation|GetRandomReachablePointinRadius (Transformation|GetActorLocation) 1e+03 0 0))))
  (AI|AIMoveTo self _output_get 0 5.0 false
    (:OnSuccess
      (Utilities|FlowControl|Delay 4.0)
      (CallFunction|MoveNPC))
    (:OnFail
      (Utilities|FlowControl|Delay 0.1)
      (CallFunction|MoveNPC))))

(event EventBeginPlay
  (CallFunction|MoveNPC))

(fn ConstructionScript)

(fn GetInvertMultiplier
  (if (Variables|Default|GetToggleInvert)
    (return -1.0)
    (else
      (return 1.0))))

(fn MoveNPC)